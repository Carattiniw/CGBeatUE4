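; Ride cart actor that, when ActiveCart is set, moves itself along the UsefulSpline of TrackRef after a start delay.
; MoveCart scales Timeline_0's play rate by Duration, applies KartStartOffset, and maps the timeline alpha to distance along the spline for world location and rotation.
; Delays chained to the timeline's Update and Finished outputs trigger reverse playback and restarts from the start.
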(event Custom|MoveCart
  ;[1 1 1] Move object along spline path
  (Utilities|FlowControl|Delay (Variables|Default|GetDelay%20Start%20Movement))
  (Components|Timeline|SetPlayRate (Variables|Default|GetTarget) (/ 1.0 (Variables|Default|GetDuration)))
  (Components|Timeline|SetNewTime (Variables|Default|GetTarget) (Variables|Default|GetKartStartOffset))
  (bind _alpha (Timeline|Timeline_0 Play)
    (:Update
      (Variables|Default|SetAlpha _alpha)
      ;;[1 1 1] Sets the location and rotation of the player character during the ride
      (Transformation|SetActorLocationAndRotation (Spline|GetLocationatDistanceAlongSpline (Variables|/Game/Blueprints/BP_SplinePath.BP_SplinePath_C|GetUsefulSpline (Variables|Default|GetTrackRef)) (Math|Float|Lerp 0.0 (Spline|GetSplineLength (Variables|/Game/Blueprints/BP_SplinePath.BP_SplinePath_C|GetUsefulSpline (Variables|Default|GetTrackRef))) (Variables|Default|GetAlpha)) "World") (Spline|GetRotationatDistanceAlongSpline (Variables|/Game/Blueprints/BP_SplinePath.BP_SplinePath_C|GetUsefulSpline (Variables|Default|GetTrackRef)) (Math|Float|Lerp 0.0 (Spline|GetSplineLength (Variables|/Game/Blueprints/BP_SplinePath.BP_SplinePath_C|GetUsefulSpline (Variables|Default|GetTrackRef))) (Variables|Default|GetAlpha)) "World"))
      (Utilities|FlowControl|Delay (Variables|Default|GetDuration))
      (Timeline|Timeline_0 ReverseFromEnd))
    (:Finished
      (Utilities|FlowControl|Delay (* (Variables|Default|GetDuration) 2.0))
      (Timeline|Timeline_0 PlayFromStart))))

(event EventBeginPlay
  ;[1 1 1] Move object along spline path
  (Utilities|FlowControl|Sequence
    (:then_0
      (if (Variables|Default|GetActiveCart)
        (CallFunction|MoveCart)))))

(event Collision|EventActorBeginOverlap
  (params (OtherActor :type Actor%20Object%20Reference)))

(fn ConstructionScript)