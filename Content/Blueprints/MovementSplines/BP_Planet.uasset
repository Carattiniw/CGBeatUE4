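; BP_Planet is an actor that spins its mesh and can travel along a referenced track's spline.
; Tick adds a per-axis relative rotation to the mesh each frame, with no delta-time scaling.
; If ActiveCart is set at BeginPlay, the CartMover timeline starts at an offset with play rate 1/Duration.
; Its alpha maps to spline distance, setting the actor's world location and rotation.
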(event Custom|MoveCart
  ;[1 1 1] Makes the object move along the spline
  (Components|Timeline|SetPlayRate (Variables|Default|GetCartMover) (/ 1.0 (Variables|Default|GetDuration)))
  (Components|Timeline|SetNewTime (Variables|Default|GetCartMover) (Variables|Default|GetKartStartOffset))
  (bind _alpha (Timeline|CartMover Play)
    (:Update
      (Variables|Default|SetAlpha _alpha)
      (Transformation|SetActorLocationAndRotation (Spline|GetLocationatDistanceAlongSpline (Variables|/Game/Blueprints/BP_SplinePath.BP_SplinePath_C|GetUsefulSpline (Variables|Default|GetTrackRef)) (Math|Float|Lerp 0.0 (Spline|GetSplineLength (Variables|/Game/Blueprints/BP_SplinePath.BP_SplinePath_C|GetUsefulSpline (Variables|Default|GetTrackRef))) (Variables|Default|GetAlpha)) "World") (Spline|GetRotationatDistanceAlongSpline (Variables|/Game/Blueprints/BP_SplinePath.BP_SplinePath_C|GetUsefulSpline (Variables|Default|GetTrackRef)) (Math|Float|Lerp 0.0 (Spline|GetSplineLength (Variables|/Game/Blueprints/BP_SplinePath.BP_SplinePath_C|GetUsefulSpline (Variables|Default|GetTrackRef))) (Variables|Default|GetAlpha)) "World")))))

(event EventBeginPlay
  ;[1 1 1] Starts the movement behavior
  (if (Variables|Default|GetActiveCart)
    (CallFunction|MoveCart)))

(event EventTick
  (params (DeltaSeconds :type Float%20%28single-precision%29))
  ;[1 1 1] Rotates Object
  (Transformation|AddRelativeRotation (Variables|Default|GetStaticMesh) (Math|Rotator|MakeRotator (Variables|Default|GetRotate%20Speed%20X) (Variables|Default|GetRotate%20Speed%20Y) (Variables|Default|GetRotate%20Speed%20Z)) false false))

(fn ConstructionScript)