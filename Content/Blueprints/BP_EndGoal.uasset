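; BP_EndGoal is an actor that travels along the spline of a referenced track; despite its name, it contains no goal logic.
; On BeginPlay, if ActiveCart is set, MoveCart starts the CartMover timeline at KartStartOffset, with play rate scaled by Duration.
; Each update maps the timeline alpha to a distance along the spline and sets the actor's world location and rotation to match.
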(event Custom|MoveCart
  (Components|Timeline|SetPlayRate (Variables|Default|GetCartMover) (/ 1.0 (Variables|Default|GetDuration)))
  (Components|Timeline|SetNewTime (Variables|Default|GetCartMover) (Variables|Default|GetKartStartOffset))
  (bind _alpha (Timeline|CartMover Play)
    (:Update
      (Variables|Default|SetAlpha _alpha)
      (Transformation|SetActorLocationAndRotation (Spline|GetLocationatDistanceAlongSpline (Variables|/Game/Blueprints/BP_SplinePath.BP_SplinePath_C|GetUsefulSpline (Variables|Default|GetTrackRef)) (Math|Float|Lerp 0.0 (Spline|GetSplineLength (Variables|/Game/Blueprints/BP_SplinePath.BP_SplinePath_C|GetUsefulSpline (Variables|Default|GetTrackRef))) (Variables|Default|GetAlpha)) "World") (Spline|GetRotationatDistanceAlongSpline (Variables|/Game/Blueprints/BP_SplinePath.BP_SplinePath_C|GetUsefulSpline (Variables|Default|GetTrackRef)) (Math|Float|Lerp 0.0 (Spline|GetSplineLength (Variables|/Game/Blueprints/BP_SplinePath.BP_SplinePath_C|GetUsefulSpline (Variables|Default|GetTrackRef))) (Variables|Default|GetAlpha)) "World")))))

(event EventBeginPlay
  (if (Variables|Default|GetActiveCart)
    (CallFunction|MoveCart)))

(event Collision|EventActorBeginOverlap
  (params (OtherActor :type Actor%20Object%20Reference)))

(fn ConstructionScript)